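; BP_Enemy_BT is an enemy Blueprint with its own health pool and a melee-style overlap attack on the player.
; Health is set on BeginPlay and reduced by AnyDamage; at zero it enables capsule physics and immediately destroys the actor.
; Overlapping DamageCollision applies damage to FPSMod1Character and prints a debug message, gated by CanDealDamage, which this graph reads but never sets.
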(event `self.ReceiveBeginPlay`
  (set `self.EnemyHealth` 600))

(event `self.ReceiveAnyDamage`
  (params (Damage :type "Float (single-precision)") (DamageType :type "DamageType Object Reference") (InstigatedBy :type "Controller Object Reference") (DamageCauser :type "Actor Object Reference"))
  (bind _output_get (set `self.RemainingDamage` (`KismetMathLibrary.FTrunc` Damage)))
  (set `self.EnemyHealth` (- (`self.EnemyHealth`) _output_get))
  (if (<= (`self.EnemyHealth`) 0)
    (`PrimitiveComponent.SetSimulatePhysics` (`self.CapsuleComponent`) true)
    (`self.K2_DestroyActor`)))

(event `self.Damage Collision.OnComponentBeginOverlap`
  (params (OverlappedComponent :type "PrimitiveComponent Object Reference") (OtherActor :type "Actor Object Reference") (OtherComp :type "PrimitiveComponent Object Reference") (OtherBodyIndex :type Integer) (bFromSweep :type Boolean) (SweepResult :type "HitResult Structure (by ref)"))
  (if (`self.Can Deal Damage`)
    (bind _asfpsmod_1character (cast `FPSMod1Character` OtherActor))
    (`GameplayStatics.ApplyDamage` _asfpsmod_1character 200.0 null null "/Script/Engine.DamageType")
    (`KismetSystemLibrary.PrintString` "Player Attacked")))

(fn `UserConstructionScript`)