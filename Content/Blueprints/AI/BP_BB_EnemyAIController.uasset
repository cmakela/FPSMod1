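; AI controller for a behavior-tree-driven enemy that tracks whether it can see the player.
; On BeginPlay it runs the behavior tree and caches the controlled BP_Enemy_BT pawn.
; Pawn sensing writes sight and target to the blackboard; a retriggerable delay of twice the sensing interval clears the sight flag once sightings stop, then halts the mutant attack montage.
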(event `self.ReceiveBeginPlay`
  (`self.RunBehaviorTree` (`self.AI Behavior Tree`))
  (bind _asbp_enemy_bt (cast `/Game/Blueprints/BP_Enemy_BT` (`self.K2_GetPawn`)))
  (set `self.Enemy BT REF` _asbp_enemy_bt))

(event `self.PawnSensing.OnSeePawn`
  (params (Pawn :type "Pawn Object Reference"))
  (bind _asfpsmod_1character (cast `FPSMod1Character` Pawn))
  (`self.Set Can See Player` true _asfpsmod_1character)
  (`KismetSystemLibrary.RetriggerableDelay` (* (`PawnSensingComponent.SensingInterval` (`self.PawnSensing`)) 2.0))
  (`self.Set Can See Player` false)
  (`AnimInstance.Montage_Stop` (`SkeletalMeshComponent.GetAnimInstance` (`Character.Mesh` (`self.Enemy BT REF`))) 0.0 "/Game/Enemy_Model/Mutant_Attack_Montage.Mutant_Attack_Montage"))

(fn `Set Can See Player`
  (params (`Can See Player` :type Boolean) (`Player Object` :type "Object Object Reference"))
  (bind _returnvalue (`AIBlueprintHelperLibrary.GetBlackboard` self))
  (if `Can See Player`
    (`BlackboardComponent.SetValueAsBool` _returnvalue "Can See Player" true)
    (`BlackboardComponent.SetValueAsObject` _returnvalue "Player Target" `Player Object`)
    (else
      (`BlackboardComponent.SetValueAsBool` _returnvalue "Can See Player" false))))

(fn `UserConstructionScript`)